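; AC_Arcetek is a building-placement component that lets the player spawn, move and rotate actors in the world.
; BeginPlay caches the owner's camera and opens the Arcetek UI with mouse cursor and Game and UI input.
; While building, Tick moves the current actor to a camera-forward trace hit, or to the trace end.
; Keys toggle build mode, clear the selection or spawn a campfire directly or via data table; the mouse wheel rotates.
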(event EventBeginPlay
  (bind _returnvalue (Game|GetPlayerController 0))
  (Utilities|FlowControl|Sequence
    (:then_0
      (Variables|Default|SetCameraComponent (Actor|GetComponentbyClass (Components|GetOwner) "/Script/Engine.CameraComponent")))
    (:then_1
      (bind _returnvalue_2 (UserInterface|CreateWidget "/Game/UserInterface/WBP_Arcetek_Main.WBP_Arcetek_Main_C" (Game|GetPlayerController 0)))
      (bind _output_get (Variables|Blueprint-Data|SetArcetekUI _returnvalue_2))
      (UserInterface|Viewport|AddtoViewport _output_get 0)
      (Input|SetInputModeGameandUI _returnvalue _output_get "DoNotLock" true false)
      (Variables|/Script/Engine.PlayerController|SetbShowMouseCursor _returnvalue true))))

(event EventTick
  (params (DeltaSeconds :type Float%20%28single-precision%29))
  (bind _currentactor (Variables|Default|GetCurrentActor))
  (bind _currentactor_2 (Variables|Default|GetCurrentActor))
  (bind _cameracomponent (Variables|Default|GetCameraComponent))
  (bind _returnvalue (Transformation|GetWorldLocation _cameracomponent))
  (if (and (Variables|Default|GetbIsBuilding) (Utilities|IsValid _currentactor))
    (bind (_outhit _returnvalue_2) (Collision|LineTraceByChannel _returnvalue (+ _returnvalue (* (Math|Vector|GetForwardVector _cameracomponent) 2.5e+03)) "TraceTypeQuery1" false (Utilities|Array|MakeArray _currentactor (Components|GetOwner)) "None" true "(R=1.000000,G=0.000000,B=0.091539,A=1.000000)"))
    (if _returnvalue_2
      (Transformation|SetActorLocation _currentactor_2 (.Location (Collision|BreakHitResult _outhit)) false false)
      (else
        (Transformation|SetActorLocation _currentactor_2 (Math|Vector|MakeVector (.x (.TraceEnd (Collision|BreakHitResult _outhit))) (.y (.TraceEnd (Collision|BreakHitResult _outhit))) (.z (.TraceEnd (Collision|BreakHitResult _outhit)))) false false)))))

(event Input|MouseEvents|MouseWheelAxis
  (params (AxisValue :type Float%20%28single-precision%29))
  (Class|ArcetekComponent|RotateActor (* AxisValue (Variables|Default|GetRotationRate))))

(event Input|KeyboardEvents|B
  (params (Key :type Key%20Structure :default "None"))
  (:Pressed
    (Utilities|FlowControl|FlipFlop
      (:A
        (Class|ArcetekComponent|EnterBuildMode true))
      (:B
        (Class|ArcetekComponent|EnterBuildMode false)))))

(event Input|KeyboardEvents|F
  (params (Key :type Key%20Structure :default "None"))
  (:Pressed
    (bind _returnvalue (Game|SpawnActorfromClass "/Game/Game/Actors/BP_Campfire.BP_Campfire_C" (Math|Transform|MakeTransform "0, 0, 0" "0, 0, 0" "1.000000,1.000000,1.000000") "Undefined" 0 0))
    (Class|ArcetekComponent|SetCurrentArcetekable _returnvalue)))

(event Input|KeyboardEvents|R
  (params (Key :type Key%20Structure :default "None"))
  (:Pressed
    (Class|ArcetekComponent|SetCurrentArcetekable)))

(event Input|KeyboardEvents|X
  (params (Key :type Key%20Structure :default "None"))
  (:Pressed
    (if (Variables|Default|GetbIsBuilding)
      (Variables|Default|GetArcetekables
        (:then
          (bind _returnvalue (Utilities|GetDataTableRow "/Game/Game/Data/Environment.Environment" "Campfire")
            (:then
              (bind _returnvalue_2 (Game|SpawnActorfromClass (.ActorClass (Utilities|Struct|BreakArcetekableData _returnvalue)) (Math|Transform|MakeTransform "0, 0, 0" "0, 0, 0" "1.000000,1.000000,1.000000") "Undefined" 0 0))
              (Class|ArcetekComponent|SetCurrentArcetekable _returnvalue_2))))
        (:else)))))