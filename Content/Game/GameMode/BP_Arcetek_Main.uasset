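; Main game mode Blueprint for Arcetek that restores the saved world and autosaves it during play.
; On BeginPlay it gets the save game from the Arcetek game instance, respawns each world data entry and loads its actor data.
; A collapsed graph then starts a looping 15-second timer that saves actors tagged "Saveable" through the game instance and prints a message on success.
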(event EventBeginPlay
  (Utilities|FlowControl|Sequence
    (:then_0
      (bind _asarcetek_game_instance (Utilities|Casting|CastToArcetekGameInstance (Game|GetGameInstance)))
      (bind _output_get (Variables|Default|SetAs%20Arcetek%20Game%20Instance _asarcetek_game_instance))
      (Variables|Default|SetArcetek%20Save%20Game (Class|ArcetekGameInstance|GetSaveGame _output_get)))
    (:then_1
      (for _array_element (Class|ArcetekSaveGame|GetWorldData (Variables|Default|GetArcetek%20Save%20Game))
        (bind _returnvalue (Game|SpawnActorfromClass (.class _array_element) (.transform _array_element) "Undefined" 0 0))
        (Class|ArcetekGameModeBase|LoadActorData _returnvalue (.data _array_element))))
    (:then_2
      (|GraphSaveGame))))

(fn ConstructionScript)

(event Custom|Save%20All%20Actors%20Event
  (bind _outactors (Actor|GetAllActorswithTag "Saveable"))
  (Class|ArcetekGameModeBase|SaveAllPlacedActors (Variables|Default|GetArcetek%20Save%20Game) _outactors)
  (bind _returnvalue (Class|ArcetekGameInstance|SaveCurrentGame (Variables|Default|GetAs%20Arcetek%20Game%20Instance)))
  (if _returnvalue
    (Development|PrintString "Game Saved")))